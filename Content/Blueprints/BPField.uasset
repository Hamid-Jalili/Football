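; Soccer field actor that detects when the ball leaves play and resets it.
; When a BPBall exits the OOBBox, its world Y against the box extent identifies a throw-in.
; Otherwise it asks the left and right Goal child actors whether the ball is inside, distinguishing goals from goal or corner kicks.
; Every outcome only prints a message, then moves the ball to just above world origin and zeroes its velocity.
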(event OnComponentEndOverlap(OOBBox)
  (params (OverlappedComponent :type Primitive%20Component%20Object%20Reference) (OtherActor :type Actor%20Object%20Reference) (OtherComp :type Primitive%20Component%20Object%20Reference) (OtherBodyIndex :type Integer))
  (bind _oob_box (Variables|Default|GetOOB%20Box))
  (bind _boxextent (Variables|/Script/Engine.BoxComponent|GetBoxExtent _oob_box))
  (bind _y (Math|Vector|BreakVector _boxextent))
  ;[1 1 1] OOB trigger
  (bind _asbpball (Utilities|Casting|CastToBPBall OtherActor))
  (if (or (> (.Y (Math|Vector|BreakVector (Transformation|GetActorLocation _asbpball))) _y) (< (.Y (Math|Vector|BreakVector (Transformation|GetActorLocation _asbpball))) (* _y -1.0)))
    (Development|PrintString "Throw in!")
    (else
      (bind _asgoal (Utilities|Casting|CastToGoal (Variables|/Script/Engine.ChildActorComponent|GetChildActor (Variables|Default|GetLeft%20Goal))))
      (bind _returnvalue (Class|Goal|IsLocationinGoal _asgoal (Transformation|GetActorLocation _asbpball)))
      (if _returnvalue
        (Development|PrintString "Golasso (Left)!")
        (else
          (bind _asgoal_2 (Utilities|Casting|CastToGoal (Variables|/Script/Engine.ChildActorComponent|GetChildActor (Variables|Default|GetRight%20Goal))))
          (bind _returnvalue_2 (Class|Goal|IsLocationinGoal _asgoal_2 (Transformation|GetActorLocation _asbpball)))
          (if _returnvalue_2
            (Development|PrintString "Golasso (Right)!")
            (else
              (Development|PrintString "Goal/Corner Kick!")))))))
  (Transformation|SetActorLocation _asbpball (Math|Vector|MakeVector 0.0 0.0 1e+01) false false)
  (Class|PrimitiveComponent|SetAllPhysicsLinearVelocity (Variables|/Script/Engine.StaticMeshActor|GetStaticMeshComponent _asbpball) "0, 0, 0" false))

(event EventBeginPlay)

(event EventActorBeginOverlap
  (params (OtherActor :type Actor%20Object%20Reference)))

(event EventTick
  (params (DeltaSeconds :type Float%20%28single-precision%29)))

(fn ConstructionScript)