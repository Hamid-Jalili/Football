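; Behavior tree node that decides whether an AI footballer should press the ball.
; Each tick it asks the footballer's team for the player closest to the ball and sets the ShouldBePressing blackboard flag only if that is this pawn.
; It also writes the ball's position to TargetLocation for every footballer, and a distance check to the ball is left unconnected.
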(event EventTick
  (params (OwnerActor :type Actor%20Object%20Reference) (DeltaSeconds :type Float%20%28single-precision%29))
  (bind _asbpfootballer (Utilities|Casting|CastToBPFootballer (Pawn|GetControlledPawn (AI|GetAIController OwnerActor))))
  (bind _returnvalue (Class|FootballTeam|GetClosestFootballertoBall (Variables|/Script/OSF.Footballer|GetTeam _asbpfootballer) (Variables|/Script/OSF.Footballer|GetBall _asbpfootballer)))
  (Class|BTFunctionLibrary|SetBlackboardValueasBool (Variables|Default|GetShouldBePressing) (== _returnvalue _asbpfootballer))
  (AI|BehaviorTree|SetBlackboardValueasVector (Variables|Default|GetTargetLocation) (Transformation|GetActorLocation (Variables|/Script/OSF.Footballer|GetBall _asbpfootballer))))