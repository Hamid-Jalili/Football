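; Goal actor that reports scores to BP_TeamGameState when a BP_Ball enters its NetTrigger, passing IsRightGoal as an integer.
; Actor hit and overlap events share a class check on Ballsack that plays force feedback for player 0.
; GetNearPostAxis picks a post by squared distance, measuring left from the goal and right from ForActor.
; It returns a Z=1 vector using the goal-to-left-post offset or the right post's world XY.
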(event OnComponentBeginOverlap(NetTrigger)
  (params (OverlappedComponent :type Primitive%20Component%20Object%20Reference) (OtherActor :type Actor%20Object%20Reference) (OtherComp :type Primitive%20Component%20Object%20Reference) (OtherBodyIndex :type Integer) (bFromSweep :type Boolean) (SweepResult :type Hit%20Result%20Structure%20%28by%20ref%29))
  (Utilities|Casting|CastToBP_Ball OtherActor)
  (bind _asbp_team_game_state (Utilities|Casting|CastToBP_TeamGameState (Game|GetGameState)))
  (Class|TeamGameState|HandleGoal _asbp_team_game_state (Math|Conversions|ToInteger(Boolean) (Variables|Default|GetIsRightGoal))))

(event Custom|OnActorHit_Event_0
  (params (SelfActor :type Actor%20Object%20Reference) (OtherActor :type Actor%20Object%20Reference) (NormalImpulse :type Vector) (Hit :type Hit%20Result%20Structure%20%28by%20ref%29))
  (if (== (Utilities|GetClass OtherActor) "/Script/OSF.Ballsack")
    (Game|Feedback|PlayDynamicForceFeedback (Game|GetPlayerController 0) 0.8 0.5 true true true true)))

(event EventBeginPlay
  (EventDispatchers|AssignOnActorHit (delegate Custom|OnActorHit_Event_0)))

(event EventActorBeginOverlap
  (params (OtherActor :type Actor%20Object%20Reference))
  (if (== (Utilities|GetClass (stale Custom|OnActorHit_Event_0 OtherActor)) "/Script/OSF.Ballsack")
    (Game|Feedback|PlayDynamicForceFeedback (Game|GetPlayerController 0) 0.8 0.5 true true true true)))

(fn ConstructionScript)

(fn GetNearPostAxis
  (params (For%20Actor :type Actor%20Object%20Reference))
  (bind _returnvalue (Transformation|GetActorLocation))
  (bind _leftpost (Variables|Default|GetLeftPost))
  (bind _rightpost (Variables|Default|GetRightPost))
  (bind _returnvalue_2 (Transformation|GetWorldLocation _leftpost))
  (bind _returnvalue_3 (Transformation|GetWorldLocation _rightpost))
  (bind _returnvalue_4 (- _returnvalue _returnvalue_2))
  (bind (_x _y) (Math|Vector|BreakVector _returnvalue_3))
  (bind (_x_2 _y_2) (Math|Vector|BreakVector _returnvalue_4))
  (if (<= (Math|Vector|VectorLengthSquared _returnvalue_4) (Math|Vector|VectorLengthSquared (- (Transformation|GetActorLocation For%20Actor) _returnvalue_3))) ; Is left post closer?
    (return (Math|Vector|MakeVector _x_2 _y_2 1.0))
    (else
      (return (Math|Vector|MakeVector _x _y 1.0)))))